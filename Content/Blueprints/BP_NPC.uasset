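; Quest NPC that talks through camera-facing floating text, shown as a skeletal mesh or a textured 2D avatar plane chosen at construction.
; Box overlap registers it on the third-person character and picks quest or completion lines by checking the string-array inventory for the needed item.
; ContinueDialogue steps through the lines; finishing completion dialogue swaps the needed item for a reward once, with a sound.
; Leaving the box hides and resets the dialogue.
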(event OnComponentBeginOverlap(Box)
  (params (OverlappedComponent :type Primitive%20Component%20Object%20Reference) (OtherActor :type Actor%20Object%20Reference) (OtherComp :type Primitive%20Component%20Object%20Reference) (OtherBodyIndex :type Integer) (bFromSweep :type Boolean) (SweepResult :type Hit%20Result%20Structure%20%28by%20ref%29))
  (bind _textrender (Variables|Default|GetTextRender))
  ;[1 1 1] Add the beginning text when we get close
  (bind _asbp_third_person_character (Utilities|Casting|CastToBP_ThirdPersonCharacter OtherActor))
  (Variables|Default|SetCharacterRef _asbp_third_person_character)
  (Variables|/Game/ThirdPerson/Blueprints/BP_ThirdPersonCharacter.BP_ThirdPersonCharacter_C|SetTalkingNPCRef _asbp_third_person_character self)
  (Variables|Default|SetQuestDone (Utilities|Array|ContainsItem (Variables|/Game/ThirdPerson/Blueprints/BP_ThirdPersonCharacter.BP_ThirdPersonCharacter_C|GetInventory (Variables|Default|GetCharacterRef)) (Variables|Default|GetItemNeeded))) ; See if we already have item
  (Rendering|SetVisibility _textrender true false)
  (Rendering|Components|TextRender|SetText _textrender (Utilities|Text|ToText(String) (Utilities|Array|Get(acopy) (select (Variables|Default|GetQuestDone) (Variables|Default|GetTextQuestDone) (Variables|Default|GetTextQuest))))))

(event OnComponentEndOverlap(Box)
  (params (OverlappedComponent :type Primitive%20Component%20Object%20Reference) (OtherActor :type Actor%20Object%20Reference) (OtherComp :type Primitive%20Component%20Object%20Reference) (OtherBodyIndex :type Integer))
  ;[1 1 1] Remove text when we go away
  (bind _asbp_third_person_character (Utilities|Casting|CastToBP_ThirdPersonCharacter OtherActor))
  (Variables|/Game/ThirdPerson/Blueprints/BP_ThirdPersonCharacter.BP_ThirdPersonCharacter_C|SetTalkingNPCRef _asbp_third_person_character 0) ; Clear the NPC Ref
  (Rendering|SetVisibility (Variables|Default|GetTextRender) false false)
  (Variables|Default|SetDialougeProgress 0))

(event Custom|ContinueDialogue
  ;[1 1 1] Continue the dialouge when left mouse is pressed
  (if (>= (+ (Variables|Default|GetDialougeProgress) 1) (Utilities|Array|Length (select (Variables|Default|GetQuestDone) (Variables|Default|GetTextQuestDone) (Variables|Default|GetTextQuest))))
    (if (Variables|Default|GetQuestDone)
      ;[1 1 1] Gives the item when quest is done
      (Utilities|FlowControl|DoOnce false
        (:Completed
          (Default|REmoveItem (Variables|Default|GetCharacterRef) (Variables|Default|GetItemNeeded))
          (Default|AddItem (Variables|Default|GetCharacterRef) (Variables|Default|GetItemgiven))
          (Audio|PlaySound2D "/Game/y2mate_com_-_Tada_sound_effect.y2mate_com_-_Tada_sound_effect" 1.0 1.0 0.0 0 0))))
    ;[1 1 1] Stop talking
    (Variables|/Game/ThirdPerson/Blueprints/BP_ThirdPersonCharacter.BP_ThirdPersonCharacter_C|SetTalkingNPCRef (Variables|Default|GetCharacterRef) 0) ; Clear the NPC Ref
    (Rendering|SetVisibility (Variables|Default|GetTextRender) false false)
    (Variables|Default|SetDialougeProgress 0)
    (else
      (bind _result (Math|Integer|IncrementInt (Variables|Default|GetDialougeProgress))
        (:%20%20
          (Rendering|Components|TextRender|SetText (Variables|Default|GetTextRender) (Utilities|Text|ToText(String) (Utilities|Array|Get(acopy) (select (Variables|Default|GetQuestDone) (Variables|Default|GetTextQuestDone) (Variables|Default|GetTextQuest)) _result))))))))

(event EventTick
  (params (DeltaSeconds :type Float%20%28single-precision%29))
  (bind _textrender (Variables|Default|GetTextRender))
  ;[1 1 1] Rotate the text so it always faces the camera
  (Transformation|SetWorldRotation _textrender (Math|Rotator|FindLookatRotation (Transformation|GetWorldLocation _textrender) (Transformation|GetActorLocation (Game|GetPlayerCameraManager 0))) false false))

(fn ConstructionScript
  (if (Variables|Default|GetUseImage)
    (Rendering|SetVisibility (Variables|Default|GetSkeletalMesh) false false)
    (Rendering|SetVisibility (Variables|Default|GetPlane) true false)
    (bind _returnvalue (Rendering|Material|CreateDynamicMaterialInstance (Variables|Default|GetPlane) 0 0 "None" :!class /Script/Engine.PrimitiveComponent))
    (Rendering|Material|SetTextureParameterValue _returnvalue "Image" (Variables|Default|Get2DAvatar))
    (else
      (Rendering|SetVisibility (Variables|Default|GetSkeletalMesh) true false)
      (Rendering|SetVisibility (Variables|Default|GetPlane) false false))))